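; Two-way teleporter pad actor that moves the player between its two pads after they stand on one for TeleportTime.
; Overlapping a pad with the player capsule starts a one-shot timer that sets the player's location to the other pad's target point.
; Leaving a pad clears the timer and the cooldown set on teleport, which guards against bouncing straight back on arrival.
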(event OnComponentBeginOverlap(Padarea1)
  (params (OverlappedComponent :type Primitive%20Component%20Object%20Reference) (OtherActor :type Actor%20Object%20Reference) (OtherComp :type Primitive%20Component%20Object%20Reference) (OtherBodyIndex :type Integer) (bFromSweep :type Boolean) (SweepResult :type Hit%20Result%20Structure%20%28by%20ref%29))
  (if (and (not (Variables|Default|GetOnCooldown)) (== OtherComp (Variables|/Script/Engine.Character|GetCapsuleComponent (Variables|Default|GetPlayerCharacter))))
    (bind _returnvalue (Utilities|Time|SetTimerbyEvent (delegate Custom|TeleportTo2) (Variables|Default|GetTeleportTime)))
    (Variables|Default|SetTeleport%20Timer _returnvalue)))

(event OnComponentBeginOverlap(Padarea2)
  (params (OverlappedComponent :type Primitive%20Component%20Object%20Reference) (OtherActor :type Actor%20Object%20Reference) (OtherComp :type Primitive%20Component%20Object%20Reference) (OtherBodyIndex :type Integer) (bFromSweep :type Boolean) (SweepResult :type Hit%20Result%20Structure%20%28by%20ref%29))
  (if (and (not (Variables|Default|GetOnCooldown)) (== OtherComp (Variables|/Script/Engine.Character|GetCapsuleComponent (Variables|Default|GetPlayerCharacter))))
    (bind _returnvalue (Utilities|Time|SetTimerbyEvent (delegate Custom|TeleportTo1) (Variables|Default|GetTeleportTime)))
    (Variables|Default|SetTeleport%20Timer _returnvalue)))

(event OnComponentEndOverlap(Padarea1)
  (params (OverlappedComponent :type Primitive%20Component%20Object%20Reference) (OtherActor :type Actor%20Object%20Reference) (OtherComp :type Primitive%20Component%20Object%20Reference) (OtherBodyIndex :type Integer))
  (if (not (Collision|IsOverlappingActor (Variables|Default|GetPadarea1) (Variables|Default|GetPlayerCharacter) :!class /Script/Engine.PrimitiveComponent))
    (Utilities|Time|ClearandInvalidateTimerbyHandle (Variables|Default|GetTeleport%20Timer))
    (Variables|Default|SetOnCooldown false)))

(event OnComponentEndOverlap(Padarea2)
  (params (OverlappedComponent :type Primitive%20Component%20Object%20Reference) (OtherActor :type Actor%20Object%20Reference) (OtherComp :type Primitive%20Component%20Object%20Reference) (OtherBodyIndex :type Integer))
  (if (not (Collision|IsOverlappingActor (Variables|Default|GetPadarea2) (Variables|Default|GetPlayerCharacter) :!class /Script/Engine.PrimitiveComponent))
    (Utilities|Time|ClearandInvalidateTimerbyHandle (Variables|Default|GetTeleport%20Timer))
    (Variables|Default|SetOnCooldown false)))

(event Custom|TeleportTo2
  (CallFunction|Teleport (Transformation|GetWorldLocation (Variables|Default|GetPadtarget2))))

(event Custom|TeleportTo1
  (CallFunction|Teleport (Transformation|GetWorldLocation (Variables|Default|GetPadtarget1))))

(event EventBeginPlay
  (bind _as0_base (Utilities|Casting|CastTo0_Base (Game|GetPlayerCharacter 0)))
  (Variables|Default|SetPlayerCharacter _as0_base))

(fn ConstructionScript)

(fn Teleport
  (params (Target :type Vector))
  (Transformation|SetActorLocation (Variables|Default|GetPlayerCharacter) Target false false)
  (Variables|Default|SetOnCooldown true))