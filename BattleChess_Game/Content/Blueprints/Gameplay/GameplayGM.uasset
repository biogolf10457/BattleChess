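; Gameplay game mode that tracks player controllers and respawns player characters.
; Controllers passed in through OnSwapPlayerControllers are added to an AllPlayerControllers array, and the logout event does nothing.
; RespawnPlayer gathers every PlayerStart, spawns the supplied character class at a randomly chosen one, and has the given controller possess it.
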(event Custom|RespawnPlayer
  (params (PlayerController :type Player%20Controller%20Object%20Reference) (PlayerCharacter :type Character%20Class%20Reference))
  ;[1 1 1] Spawn Character
  (bind _outactors (Actor|GetAllActorsOfClass "/Script/Engine.PlayerStart"))
  (Variables|GameInfo|SetSpawnPoints _outactors)
  (bind _returnvalue (Game|SpawnActorfromClass PlayerCharacter (Transformation|GetActorTransform (Utilities|Array|Get(acopy) (Variables|GameInfo|GetSpawnPoints) (Math|Random|RandomIntegerinRange 0 (- (Utilities|Array|Length (Variables|GameInfo|GetSpawnPoints)) 1)))) "Undefined" 0 0))
  (Pawn|Possess PlayerController _returnvalue))

(event EventOnSwapPlayerControllers
  (params (OldPC :type Player%20Controller%20Object%20Reference) (NewPC :type Player%20Controller%20Object%20Reference))
  ;[1 1 1] Keep Track of Connected Player Controller
  (Utilities|Array|Add (Variables|GameInfo|GetAllPlayerControllers) NewPC))

(event EventOnLogout
  (params (ExitingController :type Controller%20Object%20Reference)))

(fn ConstructionScript)