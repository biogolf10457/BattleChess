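; GameplayPC is the gameplay player controller that hands saved player settings to the server to spawn the chosen character.
; On BeginPlay, the local controller clears all widgets and loads PlayerSettings from the save slot.
; It passes them to the server-side event, which stores them and asks GameplayGM to respawn the player as the saved character.
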(event Custom|PassCharacterInfoToServer
  (params (PlayerSettingsInfo :type Player%20Info%20Structure))
  ;[1 1 1] Pass Character Info and Respawn Character
  (Variables|Default|SetPlayerSettings PlayerSettingsInfo)
  (bind _asgameplay_gm (Utilities|Casting|CastToGameplayGM (Game|GetGameMode)))
  (Default|RespawnPlayer _asgameplay_gm self (.MyPlayerCharacter (Utilities|Struct|BreakPlayerInfo (Variables|Default|GetPlayerSettings)))))

(event EventBeginPlay
  ;[1 1 1] Load Player Info and Pass to Server Side
  (if (Pawn|IsLocalController)
    (Viewport|RemoveAllWidgets)
    (CallFunction|LoadGame)
    (CallFunction|PassCharacterInfotoServer (Variables|Default|GetPlayerSettings))))

(fn ConstructionScript)

(fn LoadGame
  (bind _returnvalue (SaveGame|LoadGamefromSlot (Variables|Default|GetPlayerSettingsSave)))
  (bind _asplayer_save_game (Utilities|Casting|CastToPlayerSaveGame _returnvalue))
  (Variables|Default|SetPlayerSettings (Variables|/Game/Blueprints/AllLevels/PlayerSaveGame.PlayerSaveGame_C|GetS_PlayerInfo _asplayer_save_game)))