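; Pusher character Blueprint that can punch with a short-lived push hitbox and counts itself toward Team 1 in a score area.
; Left click attaches a PushHitBoxBP child actor in front of the character, removes it moments later, and uses CanPunch as a cooldown gate.
; Entering or leaving the first ScoreArea increments or decrements NumTeam1 on the LobbyGM game mode.
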(event Custom|CreatePushHitBox
  ;[1 1 1] Create Push Hit Box
  (if (Variables|Default|GetCanPunch)
    (Variables|Default|SetCanPunch false)
    (bind _returnvalue (AddComponent|AddChildActorComponent false (Math|Transform|MakeTransform "150.000000, 0, 0")))
    (ChildActorComponent|SetChildActorClass _returnvalue "/Game/Blueprints/Characters/PushHitBoxBP.PushHitBoxBP_C")
    (Utilities|FlowControl|Delay 0.2)
    (Components|DestroyComponent _returnvalue)
    (Utilities|FlowControl|Delay 0.8)
    (Variables|Default|SetCanPunch true)))

(event Collision|EventActorEndOverlap
  (params (OtherActor :type Actor%20Object%20Reference))
  (bind _returnvalue (Game|GetGameMode))
  (bind _aslobby_gm (Utilities|Casting|CastToLobbyGM _returnvalue))
  ;[1 1 1] Overlap first score area / update number of players in area
  (if (== OtherActor (Utilities|Array|Get(acopy) (Variables|/Game/Blueprints/Lobby/LobbyGM.LobbyGM_C|GetScoreArea _aslobby_gm)))
    (Variables|/Game/Blueprints/Lobby/LobbyGM.LobbyGM_C|SetNum_Team1 _aslobby_gm (- (Variables|/Game/Blueprints/Lobby/LobbyGM.LobbyGM_C|GetNum_Team1 _aslobby_gm) 1))))

(event Collision|EventActorBeginOverlap
  (params (OtherActor :type Actor%20Object%20Reference))
  (bind _returnvalue (Game|GetGameMode))
  (bind _aslobby_gm (Utilities|Casting|CastToLobbyGM _returnvalue))
  ;[1 1 1] Overlap first score area / update number of players in area
  (if (== OtherActor (Utilities|Array|Get(acopy) (Variables|/Game/Blueprints/Lobby/LobbyGM.LobbyGM_C|GetScoreArea _aslobby_gm)))
    (Variables|/Game/Blueprints/Lobby/LobbyGM.LobbyGM_C|SetNum_Team1 _aslobby_gm (+ (Variables|/Game/Blueprints/Lobby/LobbyGM.LobbyGM_C|GetNum_Team1 _aslobby_gm) 1))))

(event EventBeginPlay)

(event Input|MouseEvents|LeftMouseButton
  (params (Key :type Key%20Structure :default "None"))
  (:Pressed
    (CallFunction|CreatePushHitBox)))

(fn ConstructionScript
  (|CallParentFunction))