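; HealingArea is a short-lived, team-colored area actor that destroys itself a few seconds after BeginPlay through a one-shot timer.
; SetTeamAndColor stores the team and applies a red material for team one or blue for team two to both cube meshes.
; The graphs contain no healing or overlap logic, only the lifetime and team appearance.
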(event Custom|SetTeamAndColor
  (params (team :type Integer))
  (bind _output_get (Variables|Default|Setteam team))
  (switch int _output_get
    (:1
      (Rendering|Material|SetMaterial (Variables|Default|GetCube) 0 "/Game/StarterContent/Materials/Red.Red")
      (Rendering|Material|SetMaterial (Variables|Default|GetCube1) 0 "/Game/StarterContent/Materials/Red.Red"))
    (:2
      (Rendering|Material|SetMaterial (Variables|Default|GetCube) 0 "/Game/StarterContent/Materials/Blue.Blue")
      (Rendering|Material|SetMaterial (Variables|Default|GetCube1) 0 "/Game/StarterContent/Materials/Blue.Blue"))))

(event Custom|WaitForDestroy
  (Actor|DestroyActor))

(event EventBeginPlay
  (Utilities|Time|SetTimerbyEvent (delegate Custom|WaitForDestroy) 5.0))

(fn ConstructionScript)