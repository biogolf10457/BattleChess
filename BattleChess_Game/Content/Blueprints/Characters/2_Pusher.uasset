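; Pusher character Blueprint that counts toward team 2's presence in the lobby game mode's first score area.
; Begin and end overlap with that area increment or decrement NumTeam2 directly on LobbyGM, fetched by casting the current game mode.
; A left mouse press calls CreatePushHitBox with short front and back delays to perform the push.
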(event EventBeginPlay)

(event Collision|EventActorEndOverlap
  (params (OtherActor :type Actor%20Object%20Reference))
  (bind _returnvalue (Game|GetGameMode))
  (bind _aslobby_gm (Utilities|Casting|CastToLobbyGM _returnvalue))
  ;[1 1 1] Overlap first score area / update number of players in area
  (if (== OtherActor (Utilities|Array|Get(acopy) (Variables|/Game/Blueprints/Lobby/LobbyGM.LobbyGM_C|GetScoreArea _aslobby_gm)))
    (Variables|/Game/Blueprints/Lobby/LobbyGM.LobbyGM_C|SetNum_Team2 _aslobby_gm (- (Variables|/Game/Blueprints/Lobby/LobbyGM.LobbyGM_C|GetNum_Team2 _aslobby_gm) 1))))

(event EventTick
  (params (DeltaSeconds :type Float%20%28single-precision%29)))

(event Collision|EventActorBeginOverlap
  (params (OtherActor :type Actor%20Object%20Reference))
  (bind _returnvalue (Game|GetGameMode))
  (bind _aslobby_gm (Utilities|Casting|CastToLobbyGM _returnvalue))
  ;[1 1 1] Overlap first score area / update number of players in area
  (if (== OtherActor (Utilities|Array|Get(acopy) (Variables|/Game/Blueprints/Lobby/LobbyGM.LobbyGM_C|GetScoreArea _aslobby_gm)))
    (Variables|/Game/Blueprints/Lobby/LobbyGM.LobbyGM_C|SetNum_Team2 _aslobby_gm (+ (Variables|/Game/Blueprints/Lobby/LobbyGM.LobbyGM_C|GetNum_Team2 _aslobby_gm) 1))))

(event Input|MouseEvents|LeftMouseButton
  (params (Key :type Key%20Structure))
  (:Pressed
    (CallFunction|CreatePushHitBox 0.5 0.5)))

(fn ConstructionScript
  (|CallParentFunction))