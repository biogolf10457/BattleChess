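; Team 2 base Blueprint that keeps the lobby game mode's count of Team 2 actors inside score areas.
; On begin overlap with a ScoreAreaBP, it casts the game mode to LobbyGM and increments NumTeam2.
; On end overlap with a ScoreAreaBP, it decrements the same counter.
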(event Collision|EventActorBeginOverlap
  (params (OtherActor :type Actor%20Object%20Reference))
  (Utilities|Casting|CastToScoreAreaBP OtherActor)
  (bind _aslobby_gm (Utilities|Casting|CastToLobbyGM (Game|GetGameMode)))
  (Variables|/Game/Blueprints/Lobby/LobbyGM.LobbyGM_C|SetNum_Team2 _aslobby_gm (+ (Variables|/Game/Blueprints/Lobby/LobbyGM.LobbyGM_C|GetNum_Team2 _aslobby_gm) 1)))

(event Collision|EventActorEndOverlap
  (params (OtherActor :type Actor%20Object%20Reference))
  (Utilities|Casting|CastToScoreAreaBP OtherActor)
  (bind _aslobby_gm (Utilities|Casting|CastToLobbyGM (Game|GetGameMode)))
  (Variables|/Game/Blueprints/Lobby/LobbyGM.LobbyGM_C|SetNum_Team2 _aslobby_gm (- (Variables|/Game/Blueprints/Lobby/LobbyGM.LobbyGM_C|GetNum_Team2 _aslobby_gm) 1)))

(fn ConstructionScript)